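; Bicycle vehicle Blueprint controlled by an Arduino over serial, with keyboard input also supported.
; Each tick it requests a serial string and parses characters into pedal-based throttle, steering and cooldown-limited gear changes, adding movement axes to throttle and steering.
; The results drive the VehicleMovement component, while mesh socket locations for pedals, hands and seat feed the RiderAnimation instance to pose the rider.
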(event EventBeginPlay
  (Class|BikeV3Pawn|CallBeginPlay)
  ;[1 1 1] Handle Arduino connection
  (Class|ThreadBP|OpenSerial (Variables|Arduino|GetArduino%20Port) 9600)
  (bind _returnvalue (Class|ThreadBP|IsSerialPortOpen))
  (Development|PrintString "Arduino Connected!!" _returnvalue _returnvalue "(R=0.000000,G=0.660000,B=1.000000,A=1.000000)" 1e+01))

(event EventEndPlay
  (params (EndPlayReason :type EEndPlayReason%20Enum :default "Destroyed"))
  ;[1 1 1] Handle Arduino connection
  (bind _returnvalue (Class|ThreadBP|IsSerialPortOpen))
  (if _returnvalue
    (Class|ThreadBP|CloseSerial)))

(event EventTick
  (params (DeltaSeconds :type Float%20%28single-precision%29))
  (bind _vehiclemovement (Variables|Default|GetVehicleMovement))
  (bind _mesh (Variables|Character|GetMesh))
  (Class|BikeV3Pawn|CallTick DeltaSeconds)
  (Arduino|UpdateArduinoInput DeltaSeconds)
  ;[1 1 1] Update movement
  (Class|WheeledVehicleMovementComponent|SetTargetGear _vehiclemovement (Variables|Vehicle|GetTarget%20Gear) true)
  (Class|WheeledVehicleMovementComponent|SetSteeringInput _vehiclemovement (Variables|Vehicle|GetTarget%20Steering))
  (Class|WheeledVehicleMovementComponent|SetThrottleInput _vehiclemovement (Variables|Vehicle|GetTarget%20Speed))
  ;[1 1 1] Update sockets for Rider Animation
  (bind _asrider_animation (Utilities|Casting|CastToRiderAnimation (Components|SkeletalMesh|GetAnimInstance (Variables|Default|GetBike_Rider))))
  (Variables|/Script/BikeV3.RiderAnimation|Setleft_foot_position _asrider_animation (Transformation|GetSocketLocation _mesh "leftPed"))
  (Variables|/Script/BikeV3.RiderAnimation|Setright_foot_position _asrider_animation (Transformation|GetSocketLocation _mesh "rightPed"))
  (Variables|/Script/BikeV3.RiderAnimation|Setleft_hand_position _asrider_animation (Transformation|GetSocketLocation _mesh "LeftHand"))
  (Variables|/Script/BikeV3.RiderAnimation|Setright_hand_position _asrider_animation (Transformation|GetSocketLocation _mesh "RightHand"))
  (Variables|/Script/BikeV3.RiderAnimation|Setseat_position _asrider_animation (Transformation|GetSocketLocation _mesh "Seat")))

(event Input|ActionEvents|InputActionShiftUp
  (params (Key :type Key%20Structure :default "AnyKey"))
  (bind _vehiclemovement (Variables|Default|GetVehicleMovement))
  (bind _returnvalue (Class|WheeledVehicleMovementComponent|GetCurrentGear _vehiclemovement))
  ;[1 1 1] Gearing up or down with keyboard
  (:Pressed
    (if (<= (Variables|Vehicle|GetGearChangeTime) (Variables|Vehicle|GetGearDelta))
      (if (< _returnvalue (Variables|Vehicle|GetMaxGear))
        (Variables|Vehicle|SetGearDelta 0.0)
        (Variables|Vehicle|SetTarget%20Gear (+ _returnvalue 1))))))

(event Input|ActionEvents|InputActionShiftDown
  (params (Key :type Key%20Structure :default "AnyKey"))
  (bind _vehiclemovement (Variables|Default|GetVehicleMovement))
  (bind _returnvalue (Class|WheeledVehicleMovementComponent|GetCurrentGear _vehiclemovement))
  ;[1 1 1] Gearing up or down with keyboard
  (:Pressed
    (if (<= (Variables|Vehicle|GetGearChangeTime) (Variables|Vehicle|GetGearDelta))
      (if (< 0 _returnvalue)
        (Variables|Vehicle|SetGearDelta 0.0)
        (Variables|Vehicle|SetTarget%20Gear (- _returnvalue 1))))))

(fn ConstructionScript)

(fn UpdateArduinoInput
  (params (DeltaTime :type Float%20%28single-precision%29))
  ;[1 1 1] ask arduino for update
  (Class|ThreadBP|WriteSerial "e")
  (bind _returnvalue (Class|ThreadBP|ReadSerial))
  ;[1 1 1] Update components
  (Arduino|UpdateSpeedValue _returnvalue DeltaTime)
  (Arduino|UpdateSteeringValue _returnvalue)
  (Arduino|UpdateGearValue _returnvalue DeltaTime)
  (return))

(fn UpdateSpeedValue
  (params (ArduinoInput :type String) (DeltaTime :type Float%20%28single-precision%29))
  ;[1 1 1] Converter to float
  (Variables|Vehicle|SetTarget%20Speed (Math|Float|Clamp(Float) (+ (/ (* (/ (/ (Math|Conversions|ToFloat(Integer) (Utilities|String|GetSubstring ArduinoInput 4 (Utilities|String|Len ArduinoInput))) (LocalVariables|GetMaxTicks/Round)) DeltaTime) 6e+01) (Class|WheeledVehicleMovementComponent|GetEngineMaxRotationSpeed (Variables|Default|GetVehicleMovement))) (Input|AxisValues|GetMoveForward)) 0.0))
  (return))

(fn UpdateSteeringValue
  (params (Arduino%20Input :type String))
  (Variables|Vehicle|SetTarget%20Steering (Math|Float|Clamp(Float) (+ (+ (Input|AxisValues|GetMoveRight) (Math|Conversions|ToFloat(Integer) (Utilities|String|GetSubstring Arduino%20Input 1))) (* (Math|Conversions|ToFloat(Integer) (Utilities|String|GetSubstring Arduino%20Input 3)) -1.0)) -1.0))
  (return))

(fn UpdateGearValue
  (params (Arduino%20Input :type String) (Delta%20Time :type Float%20%28single-precision%29))
  (bind _returnvalue (Utilities|String|GetSubstring Arduino%20Input 2))
  (bind _returnvalue_2 (Utilities|Enum|Equal(Enum) _returnvalue "1"))
  ;[1 1 1] Check if enoguh time hae passed sinse last gear change
  (bind _output_get (Variables|Vehicle|SetGearDelta (+ (Variables|Vehicle|GetGearDelta) Delta%20Time)))
  (if (<= (Variables|Vehicle|GetGearChangeTime) _output_get)
    ;[1 1 1] increase the gear if necessary
    (if (Utilities|Enum|Equal(Enum) (Utilities|String|GetSubstring Arduino%20Input 0) "1")
      (if _returnvalue_2
        _
        (elif (< (Variables|Vehicle|GetTarget%20Gear) (Variables|Vehicle|GetMaxGear))
          (Variables|Vehicle|SetTarget%20Gear (+ (Variables|Vehicle|GetTarget%20Gear) 1))
          (Variables|Vehicle|SetGearDelta 0.0 :!label _label)
          (return)
          (else
            _)))
      (elif _returnvalue_2
        (if (< 0 (Variables|Vehicle|GetTarget%20Gear))
          (Variables|Vehicle|SetTarget%20Gear (- (Variables|Vehicle|GetTarget%20Gear) 1))
          (goto _label)
          (else
            _))))
    (return)
    (else
      (return))))