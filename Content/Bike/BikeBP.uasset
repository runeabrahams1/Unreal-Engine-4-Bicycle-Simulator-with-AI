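; Bike vehicle Blueprint driven by an Arduino controller over a serial port, opened on BeginPlay and closed on EndPlay.
; Each tick it polls the board and parses the reply's fixed character positions into gear shift and steering flags, plus a trailing tick count converted to throttle.
; Steering and throttle add the normal movement axes and are clamped, gear changes are rate-limited and bounded, and all three feed VehicleMovement.
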(event EventBeginPlay
  (Class|BikeV3Pawn|CallBeginPlay)
  (Class|ThreadBP|OpenSerial 3 9600)
  (bind _returnvalue (Class|ThreadBP|IsSerialPortOpen))
  (Development|PrintString "Arduino Connected!!" _returnvalue _returnvalue "(R=0.000000,G=0.660000,B=1.000000,A=1.000000)" 1e+01))

(event EventEndPlay
  (params (EndPlayReason :type EEndPlayReason%20Enum :default "Destroyed"))
  (Class|ThreadBP|CloseSerial))

(event EventTick
  (params (DeltaSeconds :type Float%20%28single-precision%29))
  (bind _vehiclemovement (Variables|Default|GetVehicleMovement))
  (Class|BikeV3Pawn|CallTick DeltaSeconds)
  (Arduino|UpdateArduinoInput DeltaSeconds)
  ;[1 1 1] Update movement
  (Class|WheeledVehicleMovementComponent|SetTargetGear _vehiclemovement (Variables|Arduino|GetTarget%20Gear) true)
  (Class|WheeledVehicleMovementComponent|SetSteeringInput _vehiclemovement (Variables|Arduino|GetTarget%20Steering))
  (Class|WheeledVehicleMovementComponent|SetThrottleInput _vehiclemovement (Variables|Arduino|GetTarget%20Speed)))

(fn ConstructionScript)

(fn UpdateArduinoInput
  (params (DeltaTime :type Float%20%28single-precision%29))
  ;[1 1 1] ask arduino for update
  (Class|ThreadBP|WriteSerial "e")
  (bind _returnvalue (Class|ThreadBP|ReadSerial))
  ;[1 1 1] Update components
  (Arduino|UpdateSpeedValue _returnvalue DeltaTime)
  (Arduino|UpdateSteeringValue _returnvalue)
  (Arduino|UpdateGearValue _returnvalue DeltaTime)
  (return))

(fn UpdateSpeedValue
  (params (ArduinoInput :type String) (DeltaTime :type Float%20%28single-precision%29))
  ;[1 1 1] Converter to float
  (Variables|Arduino|SetTarget%20Speed (Math|Float|Clamp(Float) (+ (/ (* (/ (/ (Math|Conversions|ToFloat(Integer) (Utilities|String|GetSubstring ArduinoInput 4 (Utilities|String|Len ArduinoInput))) (LocalVariables|GetMaxTicks/Round)) DeltaTime) 6e+01) (Class|WheeledVehicleMovementComponent|GetEngineMaxRotationSpeed (Variables|Default|GetVehicleMovement))) (Input|AxisValues|GetMoveForward)) 0.0))
  (return))

(fn UpdateSteeringValue
  (params (Arduino%20Input :type String))
  (Variables|Arduino|SetTarget%20Steering (Math|Float|Clamp(Float) (+ (+ (Input|AxisValues|GetMoveRight) (Math|Conversions|ToFloat(Integer) (Utilities|String|GetSubstring Arduino%20Input 1))) (* (Math|Conversions|ToFloat(Integer) (Utilities|String|GetSubstring Arduino%20Input 3)) -1.0)) -1.0))
  (return))

(fn UpdateGearValue
  (params (Arduino%20Input :type String) (Delta%20Time :type Float%20%28single-precision%29))
  (bind _returnvalue (Utilities|String|GetSubstring Arduino%20Input 2))
  (bind _returnvalue_2 (Utilities|Enum|Equal(Enum) _returnvalue "1"))
  ;[1 1 1] Check if enoguh time hae passed sinse last gear change
  (bind _output_get (Variables|Vehicle|SetGearDelta (+ (Variables|Vehicle|GetGearDelta) Delta%20Time)))
  (if (<= (Variables|Vehicle|GetGearChangeTime) _output_get)
    ;[1 1 1] increase the gear if necessary
    (if (Utilities|Enum|Equal(Enum) (Utilities|String|GetSubstring Arduino%20Input 0) "1")
      (if _returnvalue_2
        _
        (elif (< (Variables|Arduino|GetTarget%20Gear) (Variables|Vehicle|GetMaxGear))
          (Variables|Arduino|SetTarget%20Gear (+ (Variables|Arduino|GetTarget%20Gear) 1))
          (Variables|Vehicle|SetGearDelta 0.0 :!label _label)
          (return)
          (else
            _)))
      (elif _returnvalue_2
        (if (< 0 (Variables|Arduino|GetTarget%20Gear))
          (Variables|Arduino|SetTarget%20Gear (- (Variables|Arduino|GetTarget%20Gear) 1))
          (goto _label)
          (else
            _))))
    (return)
    (else
      (return))))